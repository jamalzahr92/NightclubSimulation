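; BP_SpeakersNS is a speaker world object whose two Niagara effects react to audio.
; On BeginPlay it finds the level's BP_AudioAnalyzer and creates a dynamic glow material instance on its mesh, which is never updated afterward.
; Every Tick it polls the analyzer and pushes volume, bass and smoothed volume into both Niagara components as user float parameters.
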(event Collision|EventActorBeginOverlap
  (params (OtherActor :type Actor%20Object%20Reference)))

(event EventTick
  (params (DeltaSeconds :type Float%20%28single-precision%29))
  (bind _audioanalyzer (Variables|Default|GetAudioAnalyzer))
  (bind _audioanalyzer_2 (Variables|Default|GetAudioAnalyzer))
  (bind _audioanalyzer_3 (Variables|Default|GetAudioAnalyzer))
  (bind _audioanalyzer_4 (Variables|Default|GetAudioAnalyzer))
  (Utilities|FlowControl|Sequence
    (:then_0
      (Class|BPIAudioReactive|GetVolume(Message) _audioanalyzer_2)
      (Niagara|SetNiagaraVariable(Float) (Variables|Default|GetNiagara) "User_Volume" (Variables|/Game/Blueprints/Actors/BP_AudioAnalyzer.BP_AudioAnalyzer_C|GetVolume _audioanalyzer_2))
      (Niagara|SetNiagaraVariable(Float) (Variables|Default|GetNiagara) "User_Bass" (Variables|/Game/Blueprints/Actors/BP_AudioAnalyzer.BP_AudioAnalyzer_C|GetTrueBass (Variables|Default|GetAudioAnalyzer)))
      (Class|BPIAudioReactive|GetSmoothedVolume(Message) _audioanalyzer_3)
      (Niagara|SetNiagaraVariable(Float) (Variables|Default|GetNiagara) "User_SmoothedVolume" (Variables|/Game/Blueprints/Actors/BP_AudioAnalyzer.BP_AudioAnalyzer_C|GetSmoothedVolume _audioanalyzer_3)))
    (:then_1
      (Class|BPIAudioReactive|GetVolume(Message) _audioanalyzer_4)
      (Niagara|SetNiagaraVariable(Float) (Variables|Default|GetNiagara1) "User_Volume" (Variables|/Game/Blueprints/Actors/BP_AudioAnalyzer.BP_AudioAnalyzer_C|GetVolume _audioanalyzer_4))
      (Niagara|SetNiagaraVariable(Float) (Variables|Default|GetNiagara1) "User_Bass" (Variables|/Game/Blueprints/Actors/BP_AudioAnalyzer.BP_AudioAnalyzer_C|GetTrueBass (Variables|Default|GetAudioAnalyzer)))
      (Class|BPIAudioReactive|GetSmoothedVolume(Message) _audioanalyzer)
      (Niagara|SetNiagaraVariable(Float) (Variables|Default|GetNiagara1) "User_SmoothedVolume" (Variables|/Game/Blueprints/Actors/BP_AudioAnalyzer.BP_AudioAnalyzer_C|GetSmoothedVolume _audioanalyzer)))))

(event EventBeginPlay
  (bind _returnvalue (Actor|GetActorOfClass "/Game/Blueprints/Actors/BP_AudioAnalyzer.BP_AudioAnalyzer_C"))
  (Variables|Default|SetAudioAnalyzer _returnvalue)
  (Rendering|Material|CreateDynamicMaterialInstance (Variables|Default|GetMesh) 0 "/Game/Materials/M_GlowMusicSpeakers.M_GlowMusicSpeakers" "None" :!class /Script/Engine.PrimitiveComponent))

(fn ConstructionScript)