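; Ambient moving-head spotlight actor that sweeps back and forth and pulses with audio.
; A ping-pong timeline swings the arms between two world rotations, mirrored by IsReversed, and nudges the head with incremental local rotation.
; Tick and OnBassUpdated both set spotlight intensity from the AudioAnalyzer's scaled smoothed volume, ignoring the bass value.
; PickNewTargetRotation is an empty stub.
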(event EventBeginPlay
  (|CallParentFunction)
  (bind _alpha (Timeline|RotationTimeline Play)
    (:Update
      (Transformation|SetWorldRotation (Variables|Default|GetSM_Robot_Wash_Arms) (Math|Rotator|Lerp(Rotator) (select (Variables|Default|GetbIsReversed) "0.000000,45.000000,0.000000" "0.000000,-45.000000,0.000000") (select (Variables|Default|GetbIsReversed) "0.000000,-45.000000,0.000000" "0.000000,45.000000,0.000000") _alpha true) false false)
      (Transformation|AddLocalRotation (Variables|Default|GetSM_Robot_Wash_Head) (Math|Rotator|Lerp(Rotator) "-0.500000,0.000000,0.000000" "0.500000,0.000000,0.000000" _alpha true) false false))
    (:Finished
      (if (Variables|Default|GetbIsGoingForward)
        (Variables|Default|SetbIsGoingForward false)
        (Timeline|RotationTimeline Reverse)
        (else
          (Variables|Default|SetbIsGoingForward true)
          (Timeline|RotationTimeline Play))))))

(event Collision|EventActorBeginOverlap
  (params (OtherActor :type Actor%20Object%20Reference))
  (|CallParentFunction OtherActor) ; This node is disabled and will not be called.\nDrag off pins to build functionality.
)

(event EventOnBassUpdated
  (params (BassValue :type Float%20%28double-precision%29))
  (bind _output_get (Variables|Default|SetCurrentIntensity (* (Variables|/Game/Blueprints/Actors/BP_AudioAnalyzer.BP_AudioAnalyzer_C|GetSmoothedVolume (Variables|Default|GetAudioAnalyzer)) 3e+02)))
  (Rendering|Components|Light|SetIntensity (Variables|Default|GetSpotLight) _output_get))

(event EventTick
  (params (DeltaSeconds :type Float%20%28single-precision%29))
  (bind _output_get (Variables|Default|SetCurrentIntensity (* (Variables|/Game/Blueprints/Actors/BP_AudioAnalyzer.BP_AudioAnalyzer_C|GetSmoothedVolume (Variables|Default|GetAudioAnalyzer)) 3e+02)))
  (Rendering|Components|Light|SetIntensity (Variables|Default|GetSpotLight) _output_get))

(fn ConstructionScript
  (|CallParentFunction))

(fn PickNewTargetRotation)