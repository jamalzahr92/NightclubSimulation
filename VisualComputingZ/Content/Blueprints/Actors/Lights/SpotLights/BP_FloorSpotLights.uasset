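; Floor spotlight actor that reacts to bass hits with a colour change, an intensity flash and a swing to a new yaw, mirrored for right-side lights.
; Tick fades the intensity and smoothly interpolates rotation toward the hit target or a cosine idle sweep, chosen by TimeSinceLastHit.
; The sweep advances by AudioAnalyzer's delta time scaled by TargetYaw.
; TimeSinceLastHit is reset on hits but never incremented here.
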(event EventBeginPlay
  (|CallParentFunction) ; This node is disabled and will not be called.\nDrag off pins to build functionality.
)

(event Collision|EventActorBeginOverlap
  (params (OtherActor :type Actor%20Object%20Reference))
  (|CallParentFunction OtherActor) ; This node is disabled and will not be called.\nDrag off pins to build functionality.
)

(event EventOnBassHit
  (params (ChosenColor :type Linear%20Color%20Structure) (TargetYaw :type Float%20%28double-precision%29) (TargetPitch :type Float%20%28double-precision%29))
  (Variables|Default|SetChosen%20Color ChosenColor)
  (bind _output_get (Variables|Default|SetTarget%20Yaw TargetYaw))
  (Variables|Default|SetYaw (select (Variables|Default|GetbIsRightSide) (* _output_get -1.0) _output_get))
  (Variables|Default|SetTargetRotationYaw (Math|Rotator|MakeRotator 0.0 0.0 (Variables|Default|GetYaw)))
  (Rendering|Components|Light|SetLightColor (Variables|Default|GetSpotLight) (Variables|Default|GetChosen%20Color) true)
  (Variables|Default|SetTimeSinceLastHit 0.0)
  (bind _output_get_2 (Variables|Default|SetCurrentIntensity 3e+04))
  (Rendering|Components|Light|SetIntensity (Variables|Default|GetSpotLight) _output_get_2))

(event EventTick
  (params (DeltaSeconds :type Float%20%28single-precision%29))
  (bind _output_get (Variables|Default|SetCurrentIntensity (Math|Interpolation|FInterpTo (Variables|Default|GetCurrentIntensity) 0.0 DeltaSeconds (Variables|Default|GetInterp%20Speed))))
  (Rendering|Components|Light|SetIntensity (Variables|Default|GetSpotLight) _output_get)
  (Variables|Default|SetSweepTime (+ (Variables|Default|GetSweepTime) (* (Variables|/Game/Blueprints/Actors/BP_AudioAnalyzer.BP_AudioAnalyzer_C|GetDeltaSeconds (Variables|Default|GetAudioAnalyzer)) (Variables|Default|GetTarget%20Yaw))))
  (bind _output_get_2 (Variables|Default|SetIdleYaw (* (Math|Trig|Cos(Radians) (Variables|Default|GetSweepTime)) (Variables|Default|GetSweepRange))))
  (Variables|Default|SetIdleRotation (Math|Rotator|MakeRotator 0.0 _output_get_2 _output_get_2))
  (bind _output_get_3 (Variables|Default|SetCurrentRotationYaw (Math|Interpolation|RInterpTo (Variables|Default|GetCurrentRotationYaw) (select (< (Variables|Default|GetTimeSinceLastHit) 1.5) (Variables|Default|GetTargetRotationYaw) (Variables|Default|GetIdleRotation)) (Variables|/Game/Blueprints/Actors/BP_AudioAnalyzer.BP_AudioAnalyzer_C|GetDeltaSeconds (Variables|Default|GetAudioAnalyzer)) 8.0)))
  (Transformation|SetWorldRotation (Variables|Default|GetSpotLight) _output_get_3 false false))

(fn ConstructionScript
  (|CallParentFunction))