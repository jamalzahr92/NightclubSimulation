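; Audio-reactive strobe spotlight fixture whose lights pulse with the sound.
; Every tick, six spotlight components get their intensity from the AudioAnalyzer peak value multiplied by a time-based sine wave.
; The construction script stacks three strobe base meshes at even spacing down the strobe arm.
; Nodes for arm rotation, procedural spotlight creation and color, emissive and beam setup are present but disconnected, so they never run.
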(event EventBeginPlay
  (|CallParentFunction) ; This node is disabled and will not be called.\nDrag off pins to build functionality.
)

(event Collision|EventActorBeginOverlap
  (params (OtherActor :type Actor%20Object%20Reference))
  (|CallParentFunction OtherActor) ; This node is disabled and will not be called.\nDrag off pins to build functionality.
)

(event EventTick
  (params (DeltaSeconds :type Float%20%28single-precision%29))
  (bind _peak (Class|BPIAudioReactive|GetPeak(Message) (Variables|Default|GetAudioAnalyzer)))
  (Rendering|Components|Light|SetIntensity (Variables|Default|GetSpotLight1) (* _peak (* (Math|Trig|Sin(Degrees) (* (Utilities|Time|GetGameTimeinSeconds) 5e+01)) 2e+02))))

(fn ConstructionScript
  (|CallParentFunction)
  (for _index (range 0 (- 3 1))
    ;[1 1 1] Mesh Creation
    (bind _returnvalue (AddComponent|AddStaticMeshComponent false (Math|Transform|MakeTransform (Math|Vector|MakeVector 0.0 0.0 (+ (* (Math|Conversions|ToFloat(Integer) _index) -2e+01) -21.0)))))
    (Transformation|AttachComponentToComponent _returnvalue (Variables|Default|GetSM_Strobe_Arm) "None" "KeepRelative" "KeepRelative" "KeepRelative" true)
    (Components|StaticMesh|SetStaticMesh _returnvalue "/Game/ModularConcertStage/Meshes/Lamps_Parts/Strobe/SM_Storbe_Base.SM_Storbe_Base")))