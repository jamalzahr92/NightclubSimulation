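; Audio-reactive actor with nine spotlights that flash in a chosen color on high-energy audio hits.
; OnHighEnergyHit recolors every light and sets its intensity from the AudioAnalyzer's smoothed high-energy value.
; Tick interpolates that intensity toward zero, so each flash fades out.
; A cosine idle-sweep rotation with a switch to a target rotation after recent hits is present but disconnected, so it never runs.
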(event EventOnHighEnergyHit
  (params (ChosenColor :type Linear%20Color%20Structure))
  (Variables|Default|SetChosen%20Color ChosenColor)
  (Rendering|Components|Light|SetLightColor (Variables|Default|GetSpotLight6) (Variables|Default|GetChosen%20Color) true)
  (Variables|Default|SetTimeSinceLastHit 0.0)
  (bind _output_get (Variables|Default|SetCurrentIntensity (* (Variables|/Game/Blueprints/Actors/BP_AudioAnalyzer.BP_AudioAnalyzer_C|GetSmoothedHighEnergy (Variables|Default|GetAudioAnalyzer)) 2e+03)))
  (Rendering|Components|Light|SetIntensity (Variables|Default|GetSpotLight4) _output_get))

(event EventTick
  (params (DeltaSeconds :type Float%20%28single-precision%29))
  (bind _output_get (Variables|Default|SetCurrentIntensity (Math|Interpolation|FInterpTo (Variables|Default|GetCurrentIntensity) 0.0 DeltaSeconds (Variables|Default|GetInterp%20Speed))))
  (Rendering|Components|Light|SetIntensity (Variables|Default|GetSpotLight6) _output_get))

(fn ConstructionScript
  (|CallParentFunction))