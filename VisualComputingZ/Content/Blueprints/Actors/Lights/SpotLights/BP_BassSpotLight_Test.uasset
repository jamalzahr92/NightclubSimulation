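; Test moving-head spotlight actor that reacts to music bass hits with color, brightness and aim changes.
; OnBassHit sets the color, scales intensity from the AudioAnalyzer's TrueBass, and sets pitch and yaw targets, mirroring yaw by side-placement flags.
; Tick fades intensity and smoothly rotates the robot head's arms for yaw and head for pitch.
; An idle sine sweep is left unconnected, though its timer still advances.
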(event EventBeginPlay
  (|CallParentFunction) ; This node is disabled and will not be called.\nDrag off pins to build functionality.
)

(event Collision|EventActorBeginOverlap
  (params (OtherActor :type Actor%20Object%20Reference))
  (|CallParentFunction OtherActor) ; This node is disabled and will not be called.\nDrag off pins to build functionality.
)

(event EventOnBassHit
  (params (ChosenColor :type Linear%20Color%20Structure) (TargetYaw :type Float%20%28double-precision%29) (TargetPitch :type Float%20%28double-precision%29))
  (Variables|Default|SetChosen%20Color ChosenColor)
  (Variables|Default|SetTarget%20Yaw TargetYaw)
  (Variables|Default|SetTargetPitch TargetPitch)
  (Variables|Default|SetYaw (select (Variables|Default|GetbIsSide) (select (Variables|Default|GetbIsRightSide) (Variables|Default|GetTarget%20Yaw) (* (Variables|Default|GetTarget%20Yaw) -1.0)) (select (Variables|Default|GetbIsRightSide) (* (Variables|Default|GetTarget%20Yaw) -1.0) (Variables|Default|GetTarget%20Yaw))))
  (Variables|Default|SetTargetRotationPitch (Math|Rotator|MakeRotator 0.0 (Variables|Default|GetTargetPitch) 0.0))
  (Variables|Default|SetTargetRotationYaw (Math|Rotator|MakeRotator 0.0 0.0 (Variables|Default|GetYaw)))
  (Rendering|Components|Light|SetLightColor (Variables|Default|GetSpotLight) (Variables|Default|GetChosen%20Color) true)
  (Variables|Default|SetTimeSinceLastHit 0.0)
  (bind _output_get (Variables|Default|SetCurrentIntensity (* (Variables|/Game/Blueprints/Actors/BP_AudioAnalyzer.BP_AudioAnalyzer_C|GetTrueBass (Variables|Default|GetAudioAnalyzer)) 2e+03)))
  (Rendering|Components|Light|SetIntensity (Variables|Default|GetSpotLight) _output_get))

(event EventTick
  (params (DeltaSeconds :type Float%20%28single-precision%29))
  (bind _output_get (Variables|Default|SetCurrentIntensity (Math|Interpolation|FInterpTo (Variables|Default|GetCurrentIntensity) 0.0 DeltaSeconds (Variables|Default|GetInterp%20Speed))))
  (Rendering|Components|Light|SetIntensity (Variables|Default|GetSpotLight) _output_get)
  (Variables|Default|SetSweepTime (+ (Variables|Default|GetSweepTime) (* (Variables|/Game/Blueprints/Actors/BP_AudioAnalyzer.BP_AudioAnalyzer_C|GetDeltaSeconds (Variables|Default|GetAudioAnalyzer)) (Variables|Default|GetTarget%20Yaw))))
  (bind _output_get_2 (Variables|Default|SetCurrentRotationYaw (Math|Interpolation|RInterpTo (Variables|Default|GetCurrentRotationYaw) (Variables|Default|GetTargetRotationYaw) (Variables|/Game/Blueprints/Actors/BP_AudioAnalyzer.BP_AudioAnalyzer_C|GetDeltaSeconds (Variables|Default|GetAudioAnalyzer)) 8.0)))
  (Transformation|SetRelativeRotation (Variables|Default|GetSM_Robot_Head_Arms) _output_get_2 false false)
  (bind _output_get_3 (Variables|Default|SetCurrentRotationPitch (Math|Interpolation|RInterpTo (Variables|Default|GetCurrentRotationPitch) (Variables|Default|GetTargetRotationPitch) (Variables|/Game/Blueprints/Actors/BP_AudioAnalyzer.BP_AudioAnalyzer_C|GetDeltaSeconds (Variables|Default|GetAudioAnalyzer)) 8.0)))
  (Transformation|SetRelativeRotation (Variables|Default|GetSM_Robot_Head_Head) _output_get_3 false false))

(fn ConstructionScript
  (|CallParentFunction))