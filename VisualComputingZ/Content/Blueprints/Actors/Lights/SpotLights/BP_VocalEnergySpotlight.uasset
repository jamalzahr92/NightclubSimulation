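; BP_VocalEnergySpotlight is a spotlight actor that flashes in a chosen color in response to vocal energy hits.
; OnVocalEnergyHit sets the light color and derives intensity from the AudioAnalyzer's smoothed vocal energy.
; Tick interpolates intensity toward zero, so each flash fades out.
; A cosine idle-sweep rotation with a switch to a target rotation after recent hits is present but never runs.
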(event EventBeginPlay
  (|CallParentFunction) ; This node is disabled and will not be called.\nDrag off pins to build functionality.
)

(event Collision|EventActorBeginOverlap
  (params (OtherActor :type Actor%20Object%20Reference))
  (|CallParentFunction OtherActor) ; This node is disabled and will not be called.\nDrag off pins to build functionality.
)

(event EventOnVocalEnergyHit
  (params (ChosenColor :type Linear%20Color%20Structure))
  (Variables|Default|SetChosen%20Color ChosenColor)
  (Rendering|Components|Light|SetLightColor (Variables|Default|GetSpotLight) (Variables|Default|GetChosen%20Color) true)
  (Variables|Default|SetTimeSinceLastHit 0.0)
  (bind _output_get (Variables|Default|SetCurrentIntensity (* (Variables|/Game/Blueprints/Actors/BP_AudioAnalyzer.BP_AudioAnalyzer_C|GetSmoothedVocalEnergy (Variables|Default|GetAudioAnalyzer)) 4e+02)))
  (Rendering|Components|Light|SetIntensity (Variables|Default|GetSpotLight) _output_get))

(event EventTick
  (params (DeltaSeconds :type Float%20%28single-precision%29))
  (bind _output_get (Variables|Default|SetCurrentIntensity (Math|Interpolation|FInterpTo (Variables|Default|GetCurrentIntensity) 0.0 DeltaSeconds (Variables|Default|GetInterp%20Speed))))
  (Rendering|Components|Light|SetIntensity (Variables|Default|GetSpotLight) _output_get))

(fn ConstructionScript
  (|CallParentFunction))