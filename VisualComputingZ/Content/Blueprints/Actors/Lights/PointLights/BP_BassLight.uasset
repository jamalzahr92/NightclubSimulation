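; BP_BassLight is a point light actor that flashes on bass hits and then fades.
; The OnBassHit event snaps the light and its tracked intensity to a fixed bright value.
; Tick eases that intensity with FInterpTo toward its unset default target of zero and applies it to the light each frame, producing a decaying pulse.
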(event EventBeginPlay
  (|CallParentFunction) ; This node is disabled and will not be called.\nDrag off pins to build functionality.
)

(event Collision|EventActorBeginOverlap
  (params (OtherActor :type Actor%20Object%20Reference))
  (|CallParentFunction OtherActor) ; This node is disabled and will not be called.\nDrag off pins to build functionality.
)

(event EventTick
  (params (DeltaSeconds :type Float%20%28single-precision%29))
  (bind _output_get (Variables|Default|SetCurrentIntensity (Math|Interpolation|FInterpTo (Variables|Default|GetCurrentIntensity) 0.0 DeltaSeconds 4.0)))
  (Rendering|Components|Light|SetIntensity (Variables|Default|GetPointLight) _output_get))

(event EventOnBassHit
  (params (ChosenColor :type Linear%20Color%20Structure) (TargetYaw :type Float%20%28double-precision%29) (TargetPitch :type Float%20%28double-precision%29))
  (Rendering|Components|Light|SetIntensity (Variables|Default|GetPointLight) 3e+03)
  (Variables|Default|SetCurrentIntensity 3e+03))

(fn ConstructionScript
  (|CallParentFunction))