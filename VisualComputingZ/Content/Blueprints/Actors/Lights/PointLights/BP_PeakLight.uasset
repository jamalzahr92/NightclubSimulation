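; BP_PeakLight is a point light actor whose brightness reacts to audio peaks.
; Every Tick, it reads the peak message from AudioAnalyzer and multiplies it by a scaled sine of game time to set the PointLight intensity.
; The unclamped sine makes the response swell and fade over time, with negative values in half of each cycle.
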(event EventBeginPlay
  (|CallParentFunction) ; This node is disabled and will not be called.\nDrag off pins to build functionality.
)

(event Collision|EventActorBeginOverlap
  (params (OtherActor :type Actor%20Object%20Reference))
  (|CallParentFunction OtherActor) ; This node is disabled and will not be called.\nDrag off pins to build functionality.
)

(event EventTick
  (params (DeltaSeconds :type Float%20%28single-precision%29))
  (bind _peak (Class|BPIAudioReactive|GetPeak(Message) (Variables|Default|GetAudioAnalyzer)))
  (Rendering|Components|Light|SetIntensity (Variables|Default|GetPointLight) (* _peak (* (Math|Trig|Sin(Degrees) (* (Utilities|Time|GetGameTimeinSeconds) 5e+01)) 4e+03))))

(fn ConstructionScript
  (|CallParentFunction))