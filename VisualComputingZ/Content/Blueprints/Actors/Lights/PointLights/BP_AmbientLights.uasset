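; BP_AmbientLights is a point light actor that pulses its brightness with the bass level of audio.
; The OnBassUpdated event scales the incoming bass value by a fixed multiplier, stores it as the current intensity and applies it to the PointLight.
; Tick is empty and the AudioAnalyzer smoothed-volume call is disconnected, so the light changes only through that event.
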(event EventBeginPlay
  (|CallParentFunction) ; This node is disabled and will not be called.\nDrag off pins to build functionality.
)

(event Collision|EventActorBeginOverlap
  (params (OtherActor :type Actor%20Object%20Reference))
  (|CallParentFunction OtherActor) ; This node is disabled and will not be called.\nDrag off pins to build functionality.
)

(event EventTick
  (params (DeltaSeconds :type Float%20%28single-precision%29)))

(event EventOnBassUpdated
  (params (BassValue :type Float%20%28double-precision%29))
  (bind _output_get (Variables|Default|SetCurrentIntensity (* BassValue 2e+03)))
  (Rendering|Components|Light|SetIntensity (Variables|Default|GetPointLight) _output_get))

(fn ConstructionScript
  (|CallParentFunction))