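; BP_LightsParent is a base actor for lights that react to audio analysis.
; On BeginPlay it finds the level's BP_AudioAnalyzer, stores it and binds handlers to its bass, vocal energy and high-frequency hit and update events.
; The handlers are empty hooks that pass values such as a chosen color, target yaw and pitch, or level values, presumably for child lights to implement.
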(event Custom|OnBassHit
  (params (ChosenColor :type Linear%20Color%20Structure) (TargetYaw :type Float%20%28double-precision%29) (TargetPitch :type Float%20%28double-precision%29)))

(event Custom|OnBassUpdated
  (params (BassValue :type Float%20%28double-precision%29)))

(event Custom|OnVocalEnergyHit
  (params (ChosenColor :type Linear%20Color%20Structure)))

(event Custom|OnHighEnergyUpdated
  (params (HighUpdated :type Float%20%28double-precision%29)))

(event Custom|OnHighEnergyHit
  (params (ChosenColor :type Linear%20Color%20Structure)))

(event EventBeginPlay
  (bind _returnvalue (Actor|GetActorOfClass "/Game/Blueprints/Actors/BP_AudioAnalyzer.BP_AudioAnalyzer_C"))
  (Variables|Default|SetAudioAnalyzer _returnvalue)
  (EventDispatchers|BindEventtoOnBassHit (Variables|Default|GetAudioAnalyzer) (delegate Custom|OnBassHit))
  (EventDispatchers|BindEventtoOnBassValueUpdated (Variables|Default|GetAudioAnalyzer) (delegate Custom|OnBassUpdated))
  (EventDispatchers|BindEventtoOnVocalEnergyHit (Variables|Default|GetAudioAnalyzer) (delegate Custom|OnVocalEnergyHit))
  (EventDispatchers|BindEventtoOnHighUpdated (Variables|Default|GetAudioAnalyzer) (delegate Custom|OnHighEnergyUpdated))
  (EventDispatchers|BindEventtoOnHighEnergyHit (Variables|Default|GetAudioAnalyzer) (delegate Custom|OnHighEnergyHit)))

(event Collision|EventActorBeginOverlap
  (params (OtherActor :type Actor%20Object%20Reference)))

(fn ConstructionScript)