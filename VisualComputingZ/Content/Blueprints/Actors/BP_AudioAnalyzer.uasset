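; Audio-reactive actor that analyzes the SM_AudioCapture submix by FFT and broadcasts band levels and hit events.
; Each tick it averages bass, mid, high and vocal magnitudes, smoothing them with fast attack and slow release.
; Rises, thresholds and cooldowns trigger hit dispatchers, most passing random palette colors; bass hits add random aim angles and, when strong, camera shake.
; A separate MicCapture envelope callback updates volume, peak and a random ambient rotation.
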(event OnAudioEnvelopeValue(MicCapture)
  (params (EnvelopeValue :type Float%20%28single-precision%29))
  (Variables|Default|SetVolume (* EnvelopeValue 3e+01))
  (Variables|Default|SetSmoothedVolume (Math|Interpolation|FInterpTo (Variables|Default|GetSmoothedVolume) (Variables|Default|GetVolume) (Utilities|Time|GetWorldDeltaSeconds) 5.0))
  (Variables|Default|SetDeltaVolume (Math|Float|Absolute(Float) (- (Variables|Default|GetVolume) (Variables|Default|GetPrevVolume))))
  (Variables|Default|SetPeak (select (> (Variables|Default|GetVolume) 1.0) 1.0 0.0))
  (Variables|Default|SetPrevVolume (Variables|Default|GetVolume))
  (Variables|Default|SetAmbientSharedRotation (Math|Rotator|MakeRotator 0.0 (Math|Random|RandomFloatinRange -9e+01 9e+01) (Math|Random|RandomFloatinRange -9e+01 9e+01))))

(event EventBeginPlay
  (Class|AudioMixerBlueprintLibrary|StartAnalyzingOutput "/Game/MetaSounds/SM_AudioCapture.SM_AudioCapture" "Large"))

(event Collision|EventActorBeginOverlap
  (params (OtherActor :type Actor%20Object%20Reference)))

(event EventTick
  (params (DeltaSeconds :type Float%20%28single-precision%29))
  (Variables|Default|SetDeltaSeconds DeltaSeconds)
  (Utilities|FlowControl|Sequence
    (:then_0
      (CallFunction|CalculateBass)
      (CallFunction|CalculateMidEnergy)
      (CallFunction|CalculateHighEnergy)
      (CallFunction|CalculateVocalEnergy)
      (CallFunction|CheckonMidHit))
    (:then_1
      (Variables|Bass|SetDeltaBass (- (Variables|Bass|GetSmoothedBass) (Variables|Bass|GetPreviousBass)))
      (Variables|Bass|SetPreviousBass (Variables|Bass|GetSmoothedBass))
      (Variables|Bass|SetBassDropCooldown (Math|Float|Max(Float) (- (Variables|Bass|GetBassDropCooldown) (Variables|Default|GetDeltaSeconds)) 0.0))
      (Variables|Default|SetHitRate (Math|Float|Max(Float) (- (Variables|Default|GetHitRate) (Variables|Default|GetDeltaSeconds)) 0.0))
      (Variables|Default|SetMidHitCooldown (Math|Float|Max(Float) (- (Variables|Default|GetMidHitCooldown) (Variables|Default|GetDeltaSeconds)) 0.0))
      (Variables|Bass|SetTrueBass (Math|Float|MapRangeClamped (Variables|Bass|GetSmoothedBass) 0.0 0.08 0.0 1.0))
      (Default|CallOnBassValueUpdated (Variables|Bass|GetTrueBass))
      (Default|CallOnHighUpdated (Math|Float|MapRangeClamped (Variables|HighEnergy|GetHighEnergy) 0.0 0.05 0.0 1.0))
      (Default|CallOnVocalUpdated (Variables|VocalEnergy|GetVocalEnergy))
      (CallFunction|OnBassHitChecks&Functionality))
    (:then_2
      (Variables|VocalEnergy|SetDeltaVocalEnergy (- (Variables|VocalEnergy|GetSmoothedVocalEnergy) (Variables|VocalEnergy|GetPreviousVocalEnergy)))
      (Variables|VocalEnergy|SetPreviousVocalEnergy (Variables|VocalEnergy|GetSmoothedVocalEnergy))
      (Variables|VocalEnergy|SetVocalEnergyCooldown (Math|Float|Max(Float) (- (Variables|VocalEnergy|GetVocalEnergyCooldown) (Variables|Default|GetDeltaSeconds)) 0.0))
      (if (Math|Boolean|ANDBoolean (> (Variables|VocalEnergy|GetDeltaVocalEnergy) 0.04) (> (Variables|VocalEnergy|GetSmoothedVocalEnergy) 1.0) (<= (Variables|VocalEnergy|GetVocalEnergyCooldown) 0.0) (< (Variables|Bass|GetSmoothedBass) 1e+01) true)
        (Variables|VocalEnergy|SetVocalEnergyCooldown 0.3)
        (Default|CallOnVocalEnergyHit (.OutItem (Utilities|Array|Random (Variables|Default|GetChosen%20Color))))))
    (:then_3
      (Variables|HighEnergy|SetDeltaHighEnergy (- (Variables|HighEnergy|GetSmoothedHighEnergy) (Variables|HighEnergy|GetPreviousHighEnergy)))
      (Variables|HighEnergy|SetPreviousHighEnergy (Variables|HighEnergy|GetSmoothedHighEnergy))
      (Variables|HighEnergy|SetHighEnergyCooldown (Math|Float|Max(Float) (- (Variables|HighEnergy|GetHighEnergyCooldown) (Variables|Default|GetDeltaSeconds)) 0.0))
      (if (Math|Boolean|ANDBoolean (> (Variables|HighEnergy|GetDeltaHighEnergy) 0.04) (> (Variables|HighEnergy|GetSmoothedHighEnergy) 0.01) (<= (Variables|HighEnergy|GetHighEnergyCooldown) 0.0) true true)
        (Variables|VocalEnergy|SetVocalEnergyCooldown 0.3)
        (Default|CallOnHighEnergyHit (.OutItem (Utilities|Array|Random (Variables|Default|GetChosen%20Color))))))))

(fn ConstructionScript)

(fn SetVolume
  (params (EnvelopeValue :type Float%20%28double-precision%29))
  (Variables|Default|SetVolume (* EnvelopeValue 3e+01)))

(fn SetSmoothedVolume
  (Variables|Default|SetSmoothedVolume (Math|Interpolation|FInterpTo (Variables|Default|GetSmoothedVolume) (Variables|Default|GetVolume) (Utilities|Time|GetWorldDeltaSeconds) 5.0)))

(fn SetDeltaVolume
  (Variables|Default|SetDeltaVolume (Math|Float|Absolute(Float) (- (Variables|Default|GetVolume) (Variables|Default|GetPrevVolume)))))

(fn SetBass)

(fn SetPrevVolume
  (Variables|Default|SetPrevVolume (Variables|Default|GetVolume)))

(fn SetPeak
  (Variables|Default|SetPeak (select (> (Variables|Default|GetVolume) 1.0) 1.0 0.0)))

(fn SetRawBass)

(fn GetMoodColor
  (if (and (> (Variables|Default|GetHitRate) 0.8) (> (Variables|HighEnergy|GetHighEnergy) 0.03))
    (return "(R=1.000000,G=0.918753,B=0.023476,A=1.000000)")
    (elif (and (> (Variables|Default|GetHitRate) 0.8) (> (Variables|Bass|GetSmoothedBass) 1.0))
      (return "(R=0.541667,G=0.035183,B=0.018111,A=1.000000)")
      (elif (and (< (Variables|Default|GetVolume) 3.0) (< (Variables|Default|GetHitRate) 0.3))
        (return "(R=0.135498,G=0.094325,B=1.000000,A=1.000000)")
        (elif (> (Variables|HighEnergy|GetHighEnergy) (Variables|Bass|GetSmoothedBass))
          (return "(R=0.093578,G=1.000000,B=0.000000,A=1.000000)")
          (else
            (return "(R=1.000000,G=1.000000,B=1.000000,A=1.000000)")))))))

(fn CalculateBass
  ;[0.15 0.15 0.15 0.5] Gathers the Magnitude Frequencies of Bass, averages it and interpolates it to get SmoothedBass
  (bind _magnitudes (Class|AudioMixerBlueprintLibrary|GetMagnitudeforFrequencies (Variables|Frequencies|GetBassFrequencies) "/Game/MetaSounds/SM_AudioCapture.SM_AudioCapture"))
  (Variables|Bass|SetRawBassSum 0.0)
  (for _array_element _magnitudes
    (Variables|Bass|SetRawBassSum (+ _array_element (Variables|Bass|GetRawBassSum))))
  (bind _output_get (Variables|Bass|SetBassEnergy (/ (Variables|Bass|GetRawBassSum) (Utilities|Array|Length (Variables|Frequencies|GetBassFrequencies)))))
  (Variables|Bass|SetSmoothedBass (Math|Interpolation|FInterpTo (Variables|Bass|GetSmoothedBass) _output_get (Variables|Default|GetDeltaSeconds) (select (> (Variables|Bass|GetBassEnergy) (Variables|Bass|GetSmoothedBass)) 2e+01 4.0))))

(fn CalculateMidEnergy
  ;[0.15 0.15 0.15 0.5] Gathers the Magnitude Frequencies of mid energy, averages it and interpolates it to get SmoothedMidEnergy
  (bind _magnitudes (Class|AudioMixerBlueprintLibrary|GetMagnitudeforFrequencies (Variables|Frequencies|GetMidFrequencies) "/Game/MetaSounds/SM_AudioCapture.SM_AudioCapture"))
  (Variables|MidEnergy|SetMidEnergySum 0.0)
  (for _array_element _magnitudes
    (Variables|MidEnergy|SetMidEnergySum (+ _array_element (Variables|MidEnergy|GetMidEnergySum))))
  (Variables|MidEnergy|SetMidEnergy (/ (Variables|MidEnergy|GetMidEnergySum) (Utilities|Array|Length (Variables|Frequencies|GetMidFrequencies))))
  (Variables|MidEnergy|SetSmoothedMidEnergy (Math|Interpolation|FInterpTo (Variables|MidEnergy|GetSmoothedMidEnergy) (Variables|MidEnergy|GetMidEnergy) (Variables|Default|GetDeltaSeconds) (select (> (Variables|MidEnergy|GetMidEnergy) (Variables|MidEnergy|GetSmoothedMidEnergy)) 2e+01 4.0))))

(fn CalculateHighEnergy
  ;[0.15 0.15 0.15 0.5] Gathers the Magnitude Frequencies of high energy, averages it and interpolates it to get SmoothedHighEnergy
  (bind _magnitudes (Class|AudioMixerBlueprintLibrary|GetMagnitudeforFrequencies (Variables|Frequencies|GetHighFrequencies) "/Game/MetaSounds/SM_AudioCapture.SM_AudioCapture"))
  (Variables|HighEnergy|SetHighEnergySum 0.0)
  (for _array_element _magnitudes
    (Variables|HighEnergy|SetHighEnergySum (+ _array_element (Variables|HighEnergy|GetHighEnergySum))))
  (Variables|HighEnergy|SetHighEnergy (/ (Variables|HighEnergy|GetHighEnergySum) (Utilities|Array|Length (Variables|Frequencies|GetHighFrequencies))))
  (Variables|HighEnergy|SetSmoothedHighEnergy (Math|Interpolation|FInterpTo (Variables|HighEnergy|GetSmoothedHighEnergy) (Variables|HighEnergy|GetHighEnergy) (Variables|Default|GetDeltaSeconds) (select (> (Variables|HighEnergy|GetHighEnergy) (Variables|HighEnergy|GetSmoothedHighEnergy)) 2e+01 4.0))))

(fn CalculateVocalEnergy
  (bind _magnitudes (Class|AudioMixerBlueprintLibrary|GetMagnitudeforFrequencies (Variables|Frequencies|GetVocalFrequencies) "/Game/MetaSounds/SM_AudioCapture.SM_AudioCapture"))
  (Variables|VocalEnergy|SetVocalEnergySum 0.0)
  (for _array_element _magnitudes
    (Variables|VocalEnergy|SetVocalEnergySum (+ _array_element (Variables|VocalEnergy|GetVocalEnergySum))))
  (Variables|VocalEnergy|SetVocalEnergy (/ (Variables|VocalEnergy|GetVocalEnergySum) (Utilities|Array|Length (Variables|Frequencies|GetVocalFrequencies))))
  (Variables|VocalEnergy|SetSmoothedVocalEnergy (Math|Interpolation|FInterpTo (Variables|VocalEnergy|GetSmoothedVocalEnergy) (Variables|VocalEnergy|GetVocalEnergy) (Variables|Default|GetDeltaSeconds) (select (> (Variables|VocalEnergy|GetVocalEnergy) (Variables|VocalEnergy|GetSmoothedVocalEnergy)) 2e+01 4.0))))

(fn CheckonMidHit
  (if (Math|Boolean|ANDBoolean (> (Variables|MidEnergy|GetMidEnergy) 0.0) (> (Variables|HighEnergy|GetHighEnergy) 0.0) (> (Variables|Bass|GetBassDropCooldown) 0.1) (<= (Variables|Default|GetMidHitCooldown) 0.0))
    (Variables|Default|SetMidHitCooldown 0.2)
    (Default|CallOnMidHit)))

(fn OnBassHitChecks&Functionality
  (if (Math|Boolean|ANDBoolean (> (Variables|Bass|GetDeltaBass) 0.04) (> (Variables|Bass|GetSmoothedBass) 1e+01) (<= (Variables|Bass|GetBassDropCooldown) 0.0) true true)
    (Variables|Bass|SetBassDropCooldown 0.3)
    (Variables|Default|SetHitRate 1.0)
    (Variables|Bass|SetBassSharedYaw (Math|Random|RandomFloatinRange -6e+01 -3e+01))
    (Variables|Bass|SetBassSharedPitch (Math|Random|RandomFloatinRange -1.5e+02 -1.1e+02))
    (CallFunction|GetMoodColor)
    (Default|CallOnBassHit (.OutItem (Utilities|Array|Random (Variables|Default|GetChosen%20Color))) (Variables|Bass|GetBassSharedYaw) (Variables|Bass|GetBassSharedPitch))
    (if (> (Variables|Bass|GetSmoothedBass) 3e+01)
      (Game|Feedback|ClientStartCameraShake (Game|GetPlayerController 0) "/Game/Blueprints/BP_CameraShake.BP_CameraShake_C" (Math|Float|MapRangeClamped (Variables|Bass|GetSmoothedBass) 0.3 1.0 0.5 2.0) "CameraLocal" "0, 0, 0"))))

(fn GetBass
  (return (Variables|Default|GetBass)))

(fn GetPeak
  (return (Variables|Default|GetPeak)))

(fn GetSmoothedVolume
  (return (Variables|Default|GetSmoothedVolume)))

(fn GetVolume
  (return (Variables|Default|GetVolume)))