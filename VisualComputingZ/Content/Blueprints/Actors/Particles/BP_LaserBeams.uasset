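; BP_LaserBeams is an audio-reactive effect actor that fires short Niagara laser bursts on bass hits.
; On BeginPlay it finds BP_AudioAnalyzer and binds to its bass-hit and high-frequency events; the latter handler is empty.
; Each hit activates Niagara, maps SmoothedBass to spawn rate, randomizes root roll and pitch, then deactivates after a brief delay.
; The hit's color and target angle parameters go unused.
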(event Custom|OnBassHit
  (params (ChosenColor :type Linear%20Color%20Structure) (TargetYaw :type Float%20%28double-precision%29) (TargetPitch :type Float%20%28double-precision%29))
  (if true
    (Components|Activation|Activate (Variables|Default|GetNiagara) true)
    (Niagara|SetNiagaraVariable(Float) (Variables|Default|GetNiagara) "User.SpawnRate" (Math|Float|MapRangeClamped (Variables|/Game/Blueprints/Actors/BP_AudioAnalyzer.BP_AudioAnalyzer_C|GetSmoothedBass (Variables|Default|GetAudioAnalyzer)) 0.3 1.0 5e+01 1.5e+02))
    (Transformation|SetRelativeRotation (Variables|Default|GetDefaultSceneRoot) (Math|Rotator|MakeRotator (Math|Random|RandomFloatinRange 0.0 3.6e+02) (Math|Random|RandomFloatinRange 0.0 3.6e+02) 0.0) false false)
    (Utilities|FlowControl|Delay 0.01)
    (Components|Activation|Deactivate (Variables|Default|GetNiagara))))

(event Custom|OnHighPitch
  (params (HighUpdated :type Float%20%28double-precision%29)))

(event EventBeginPlay
  (bind _returnvalue (Actor|GetActorOfClass "/Game/Blueprints/Actors/BP_AudioAnalyzer.BP_AudioAnalyzer_C"))
  (bind _output_get (Variables|Default|SetAudioAnalyzer _returnvalue))
  (EventDispatchers|BindEventtoOnBassHit _output_get (delegate Custom|OnBassHit))
  (EventDispatchers|BindEventtoOnHighUpdated _output_get (delegate Custom|OnHighPitch)))

(event Collision|EventActorBeginOverlap
  (params (OtherActor :type Actor%20Object%20Reference)))

(event EventTick
  (params (DeltaSeconds :type Float%20%28single-precision%29)))

(fn ConstructionScript)