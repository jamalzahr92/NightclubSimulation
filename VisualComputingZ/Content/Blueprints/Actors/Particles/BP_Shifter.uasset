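; BP_Shifter is an audio-reactive particle actor that drives its Niagara effect from the bass in the analyzed audio.
; Each Tick it reads the AudioAnalyzer and writes TrueBass to the User_SmoothedBass parameter when SmoothedBass clears a fixed threshold, otherwise zero.
; Smoothed bass therefore only gates the effect, while true bass sets its strength.
; The OnBassHit event is empty, and the volume and vocal-energy parameter writes are unconnected.
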(event EventBeginPlay
  (|CallParentFunction))

(event Collision|EventActorBeginOverlap
  (params (OtherActor :type Actor%20Object%20Reference))
  (|CallParentFunction OtherActor) ; This node is disabled and will not be called.\nDrag off pins to build functionality.
)

(event EventTick
  (params (DeltaSeconds :type Float%20%28single-precision%29))
  (bind _audioanalyzer (Variables|Default|GetAudioAnalyzer))
  (if (> (Variables|/Game/Blueprints/Actors/BP_AudioAnalyzer.BP_AudioAnalyzer_C|GetSmoothedBass _audioanalyzer) 1e+01)
    (Niagara|SetNiagaraVariable(Float) (Variables|Default|GetNiagara) "User_SmoothedBass" (Variables|/Game/Blueprints/Actors/BP_AudioAnalyzer.BP_AudioAnalyzer_C|GetTrueBass _audioanalyzer))
    (else
      (Niagara|SetNiagaraVariable(Float) (Variables|Default|GetNiagara) "User_SmoothedBass" 0.0))))

(event EventOnBassHit
  (params (ChosenColor :type Linear%20Color%20Structure) (TargetYaw :type Float%20%28double-precision%29) (TargetPitch :type Float%20%28double-precision%29)))

(fn ConstructionScript
  (|CallParentFunction))