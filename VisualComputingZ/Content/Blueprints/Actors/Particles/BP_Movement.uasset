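; Audio-reactive particle actor that drives a Niagara effect from an audio analyzer.
; Each Tick it reads volume, bass and smoothed volume from AudioAnalyzer and writes them to the Niagara user float parameters.
; Bass comes from the analyzer's SmoothedBass variable after a GetBassMessage call, whose return value is unused.
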(event EventBeginPlay
  (|CallParentFunction) ; This node is disabled and will not be called.\nDrag off pins to build functionality.
)

(event Collision|EventActorBeginOverlap
  (params (OtherActor :type Actor%20Object%20Reference))
  (|CallParentFunction OtherActor) ; This node is disabled and will not be called.\nDrag off pins to build functionality.
)

(event EventTick
  (params (DeltaSeconds :type Float%20%28single-precision%29))
  (bind _audioanalyzer (Variables|Default|GetAudioAnalyzer))
  (bind _volume (Class|BPIAudioReactive|GetVolume(Message) (Variables|Default|GetAudioAnalyzer)))
  (Niagara|SetNiagaraVariable(Float) (Variables|Default|GetNiagara) "User_Volume" _volume)
  (Class|BPIAudioReactive|GetBass(Message) _audioanalyzer)
  (Niagara|SetNiagaraVariable(Float) (Variables|Default|GetNiagara) "User_Bass" (Variables|/Game/Blueprints/Actors/BP_AudioAnalyzer.BP_AudioAnalyzer_C|GetSmoothedBass _audioanalyzer))
  (bind _smoothedvolume (Class|BPIAudioReactive|GetSmoothedVolume(Message) (Variables|Default|GetAudioAnalyzer)))
  (Niagara|SetNiagaraVariable(Float) (Variables|Default|GetNiagara) "User_SmoothedVolume" _smoothedvolume))

(fn ConstructionScript
  (|CallParentFunction))