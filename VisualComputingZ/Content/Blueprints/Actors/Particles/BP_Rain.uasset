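; BP_Rain is a rain particle actor whose Niagara effect reacts to analyzed audio.
; Every Tick it queries an AudioAnalyzer through interface messages for volume, bass and smoothed volume.
; It writes those values straight into Niagara user float parameters, leaving any visual response to the particle system.
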(event EventBeginPlay
  (|CallParentFunction) ; This node is disabled and will not be called.\nDrag off pins to build functionality.
)

(event Collision|EventActorBeginOverlap
  (params (OtherActor :type Actor%20Object%20Reference))
  (|CallParentFunction OtherActor) ; This node is disabled and will not be called.\nDrag off pins to build functionality.
)

(event EventTick
  (params (DeltaSeconds :type Float%20%28single-precision%29))
  (bind _audioanalyzer (Variables|Default|GetAudioAnalyzer))
  (bind _audioanalyzer_2 (Variables|Default|GetAudioAnalyzer))
  (Class|BPIAudioReactive|GetVolume(Message) _audioanalyzer_2)
  (Niagara|SetNiagaraVariable(Float) (Variables|Default|GetNiagara) "User_Volume" (Variables|/Game/Blueprints/Actors/BP_AudioAnalyzer.BP_AudioAnalyzer_C|GetVolume _audioanalyzer_2))
  (Niagara|SetNiagaraVariable(Float) (Variables|Default|GetNiagara) "User_Bass" (Variables|/Game/Blueprints/Actors/BP_AudioAnalyzer.BP_AudioAnalyzer_C|GetTrueBass (Variables|Default|GetAudioAnalyzer)))
  (Class|BPIAudioReactive|GetSmoothedVolume(Message) _audioanalyzer)
  (Niagara|SetNiagaraVariable(Float) (Variables|Default|GetNiagara) "User_SmoothedVolume" (Variables|/Game/Blueprints/Actors/BP_AudioAnalyzer.BP_AudioAnalyzer_C|GetSmoothedVolume _audioanalyzer)))

(fn ConstructionScript
  (|CallParentFunction))