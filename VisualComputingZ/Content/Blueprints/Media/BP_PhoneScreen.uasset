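; BP_PhoneScreen is a Blueprint for phone-stream media playback that currently only serves as a capture device probe.
; On BeginPlay it enumerates video capture devices and prints each display name and URL on screen.
; Several unconnected experiments open PhoneMediaPlayer from StreamURL or the CAP_PhoneStream source, some with delayed Play calls and debug prints, but none of them run.
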(event EventBeginPlay
  (bind _outdevices (Class|MediaBlueprintFunctionLibrary|EnumerateVideoCaptureDevices -1))
  (for _array_element _outdevices
    (Development|PrintString (Utilities|String|ToString(Text) (.DisplayName (Utilities|Struct|BreakMediaCaptureDevice _array_element))) true true "(R=0.000000,G=0.660000,B=1.000000,A=1.000000)" 1e+02)
    (Development|PrintString (.Url (Utilities|Struct|BreakMediaCaptureDevice _array_element)) true true "(R=0.000000,G=0.660000,B=1.000000,A=1.000000)" 1e+02)))

(event Collision|EventActorBeginOverlap
  (params (OtherActor :type Actor%20Object%20Reference)))

(event EventTick
  (params (DeltaSeconds :type Float%20%28single-precision%29)))

(fn ConstructionScript)