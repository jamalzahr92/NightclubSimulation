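; Construction-script driven ellipsoidal stage lamp for a modular concert stage, with no active runtime logic.
; Exposed rotation values swivel the hanger, tilt the light body and angle four barn-door flaps.
; Light color and intensity feed both a dynamic emissive material on the lamp mesh and the SpotLight.
; A beam intensity value sets the SpotLight's volumetric scattering.
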(event EventBeginPlay)

(event Collision|EventActorBeginOverlap
  (params (OtherActor :type Actor%20Object%20Reference)))

(event EventTick
  (params (DeltaSeconds :type Float%20%28single-precision%29)))

(fn ConstructionScript
  (bind _light_intensity (Variables|Default|GetLight_Intensity))
  (bind _spotlight (Variables|Default|GetSpotLight))
  (bind _sm_ellipsoidal_light (Variables|Default|GetSM_Ellipsoidal_Light))
  (bind _light_color (Variables|Default|GetLight_Color))
  (Transformation|SetRelativeRotation (Variables|Default|GetSM_Ellipsoidal_Hanger) (Math|Rotator|MakeRotator 0.0 0.0 (Variables|Default|GetVertical_Rotation)) false false)
  (Transformation|SetRelativeRotation _sm_ellipsoidal_light (Math|Rotator|MakeRotator 0.0 (Variables|Default|GetHorizontal_Rotation%20%28Up%20and%20Down%29) 0.0) false false)
  (Transformation|AddLocalRotation (Variables|Default|GetSM_Ellipsoidal_Barn_Door) (Math|Rotator|MakeRotator (* (Variables|Default|GetBarn_Door_Rotation) -1.0) 0.0 0.0) false false)
  (bind _returnvalue (Rendering|Material|CreateDynamicMaterialInstance _sm_ellipsoidal_light 1 "/Game/ModularConcertStage/Materials/Instances/MI_Light_Emissive_Ellipsoidal.MI_Light_Emissive_Ellipsoidal" "None" :!class /Script/Engine.PrimitiveComponent))
  (Rendering|Material|SetVectorParameterValue _returnvalue "Light_Color" _light_color :!class /Script/Engine.MaterialInstanceDynamic)
  (Rendering|Material|SetScalarParameterValue _returnvalue "Light_Emissive_Intensity" (/ _light_intensity 1e+03) :!class /Script/Engine.MaterialInstanceDynamic)
  (Rendering|Components|Light|SetLightColor _spotlight _light_color true)
  (Rendering|Components|Light|SetIntensity _spotlight _light_intensity)
  (Class|LightComponent|SetVolumetricScatteringIntensity _spotlight (Variables|Default|GetLight%20Beam%20Intensity)))